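; AI character Blueprint that can use objects and can itself be used by other actors to accumulate a displayed value.
; UseObject plays the TopDownUse montage behind a DoOnce that resets after a delay of the montage's length.
; Used adds the incoming value to its own, clears IsUsable and updates the ValueDisplay text.
; CanUse? reports IsUsable to the querying actor.
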(event EventUseObject
  (params (UsedObject :type Actor%20Object%20Reference))
  ;[1 1 1] Do animation when user is using object
  (Utilities|FlowControl|DoOnce false :!label _label
    (:Completed
      (bind _returnvalue (Animation|PlayAnimMontage "/Game/Mannequin/Animations/TopDownUse_Montage.TopDownUse_Montage" 1.0 "None"))
      (Utilities|FlowControl|Delay _returnvalue)
      (goto _label Reset))))

(event EventUsed
  (params (UsingActor :type Actor%20Object%20Reference) (Value :type Integer))
  ;[1 1 1] Set ValueDisplay once usable thing is used
  (bind _output_get (Variables|Default|SetValue (+ Value (Variables|Default|GetValue))))
  (Variables|Default|SetIsUsable false)
  (Rendering|Components|TextRender|SetText (Variables|Default|GetValueDisplay) (Utilities|Text|ToText(Integer) _output_get)))

(fn ConstructionScript)

(fn CanUse?
  (params (UsingActor :type Actor%20Object%20Reference))
  (return (Variables|Default|GetIsUsable)))